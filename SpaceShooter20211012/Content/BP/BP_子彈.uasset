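; Bullet actor Blueprint (子彈) that moves with a ProjectileMovement component and has configurable color, size and speed.
; The construction script creates a dynamic material on the bullet component, sets that component's world scale from 尺寸 and copies 子彈速度 into both max and initial speed.
; On BeginPlay it applies the 顏色 variable to the material's color vector parameter.
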(event `self.ReceiveBeginPlay`
  ;[0.5729 0.1373 0.1373] 材質設定
  (`MaterialInstanceDynamic.SetVectorParameterValue` (`self.子彈材質球`) "顏色" (`self.顏色`)))

(fn `UserConstructionScript`
  (bind _projectilemovement (`self.ProjectileMovement`))
  (bind _returnvalue (`PrimitiveComponent.CreateDynamicMaterialInstance` (`self.子彈`) 0 null "None"))
  (set `self.子彈材質球` _returnvalue)
  (`SceneComponent.SetWorldScale3D` (`self.子彈`) (`self.尺寸`))
  (bind _output_get (set `ProjectileMovementComponent.MaxSpeed` (`self.子彈速度`) _projectilemovement))
  (set `ProjectileMovementComponent.InitialSpeed` _output_get _projectilemovement))